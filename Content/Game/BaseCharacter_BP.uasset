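; BaseCharacter_BP is a player character Blueprint handling movement, camera look, jumping, running and crouching.
; Input axes drive movement and controller rotation, while actions call Jump, toggle crouch, and raise MaxWalkSpeed while Run is held.
; A camera-direction line trace meant to briefly swap a looked-at TowerArea's material is present but disconnected, as Tick is empty.
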(event `InputAxis|Forward_Backward`
  (params (AxisValue :type "Float (single-precision)"))
  ;[1 1 1] Axis Movement Left and Right
  (`self.AddMovementInput` (`self.GetActorForwardVector`) AxisValue))

(event `InputAxis|Rotate_Left_Right`
  (params (AxisValue :type "Float (single-precision)"))
  ;[1 1 1] Player Rotate Left, Right, Up, Down
  (`self.AddControllerYawInput` AxisValue))

(event `InputAxis|Look_Up_Down`
  (params (AxisValue :type "Float (single-precision)"))
  ;[1 1 1] Player Rotate Left, Right, Up, Down
  (`self.AddControllerPitchInput` AxisValue))

(event `InputAxis|Left_Right`
  (params (AxisValue :type "Float (single-precision)"))
  ;[1 1 1] Axis Movement Left and Right
  (`self.AddMovementInput` (`self.GetActorRightVector`) AxisValue))

(event `InputAction|Jump`
  (params (Key :type "Key Structure"))
  ;[1 1 1] Player Run
  (:`Pressed`
    (`self.Jump`)))

(event `InputAction|Run`
  (params (Key :type "Key Structure"))
  (bind _charactermovement (`self.CharacterMovement`))
  ;[1 1 1] Player Run
  (:`Pressed`
    (set `CharacterMovementComponent.MaxWalkSpeed` 900.0 _charactermovement))
  (:`Released`
    (set `CharacterMovementComponent.MaxWalkSpeed` 600.0 _charactermovement)))

(event `InputAction|Crouch`
  (params (Key :type "Key Structure"))
  ;[1 1 1] Player Crouch
  (:`Pressed`
    (`self.Crouch`))
  (:`Released`
    (`self.UnCrouch`)))

(event `self.ReceiveTick`
  (params (DeltaSeconds :type "Float (single-precision)"))
  ;[1 1 1] Is Character Looking at Tower Area
)

(fn `UserConstructionScript`)